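; Side-view camera actor that follows a target along X and Z while keeping its Y fixed.
; Each tick, UpdateCamera eases X toward the target through a dead zone.
; Z eases toward target height plus HeightOffset, minus that offset clamped between negative FollowSpeedZ and DeadZoneZ, independent of camera height.
; SetFollowTarget falls back to PreviewTarget for invalid pawns and snaps the camera on the first valid target only.
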(event EventBeginPlay)

(event Collision|EventActorBeginOverlap
  (params (OtherActor :type Actor%20Object%20Reference)))

(event EventTick
  (params (DeltaSeconds :type Float%20%28single-precision%29))
  (Utilities|IsValid (Variables|Default|GetFollowTarget)
    (:Is%20Valid
      (CallFunction|UpdateCamera DeltaSeconds false))))

(fn ConstructionScript)

(fn UpdateCamera
  (params (DeltaSeconds :type Float%20%28double-precision%29) (Snap :type Boolean))
  (bind _returnvalue (Transformation|GetActorLocation))
  (bind _followtarget (Variables|Default|GetFollowTarget))
  (bind _heightoffset (Variables|Default|GetHeightOffset))
  (bind _deadzonex (Variables|Default|GetDeadZoneX))
  (bind _returnvalue_2 (Transformation|GetActorLocation _followtarget))
  (bind _returnvalue_3 (+ (.z _returnvalue_2) _heightoffset))
  (Transformation|SetActorLocation (Math|Vector|MakeVector (Math|Float|SelectFloat (.x _returnvalue_2) (Math|Interpolation|FInterpTo (.x _returnvalue) (- (.x _returnvalue_2) (Math|Float|Clamp(Float) (- (.x _returnvalue_2) (.x _returnvalue)) (* _deadzonex -1.0) _deadzonex)) DeltaSeconds (Variables|Default|GetFollowSpeedX)) Snap) (.y _returnvalue) (Math|Float|SelectFloat _returnvalue_3 (Math|Interpolation|FInterpTo (.z _returnvalue) (- _returnvalue_3 (Math|Float|Clamp(Float) (- _returnvalue_3 (.z _returnvalue_2)) (* (Variables|Default|GetFollowSpeedZ) -1.0) (Variables|Default|GetDeadZoneZ))) DeltaSeconds (Variables|Default|GetFollowSpeedZ)) Snap)) false false))

(fn SetFollowTarget
  (params (NewPawn :type Pawn%20Object%20Reference))
  (Utilities|IsValid NewPawn
    (:Is%20Valid
      (Variables|Default|SetFollowTarget NewPawn))
    (:Is%20Not%20Valid
      (Variables|Default|SetFollowTarget (Variables|Default|GetPreviewTarget))))
  (if (not (Variables|Default|GetHasInitialFrame))
    (Utilities|IsValid (Variables|Default|GetFollowTarget)
      (:Is%20Valid
        (CallFunction|UpdateCamera 0.0 true)
        (Variables|Default|SetHasInitialFrame true)))))