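; Blockout hinged door that the player opens and closes, with swing direction set by the player's facing.
; InteractZone overlaps set or clear the player character's DoorInRange reference to this door.
; OpenDoor alternates playing and reversing a timeline that yaws the Hinge, fixing the swing sign from PlayerFacingX on each opening.
; DoorBlocker collision turns off as opening starts and returns only once the door finishes closing.
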(event OnComponentBeginOverlap(InteractZone)
  (params (OverlappedComponent :type Primitive%20Component%20Object%20Reference) (OtherActor :type Actor%20Object%20Reference) (OtherComp :type Primitive%20Component%20Object%20Reference) (OtherBodyIndex :type Integer) (bFromSweep :type Boolean) (SweepResult :type Hit%20Result%20Structure%20%28by%20ref%29))
  (bind _asbp_player_character (Utilities|Casting|CastToBP_PlayerCharacter OtherActor))
  (Variables|/Game/BLUE_PRINTS/BP_PlayerCharacter.BP_PlayerCharacter_C|SetDoorInRange _asbp_player_character self))

(event OnComponentEndOverlap(InteractZone)
  (params (OverlappedComponent :type Primitive%20Component%20Object%20Reference) (OtherActor :type Actor%20Object%20Reference) (OtherComp :type Primitive%20Component%20Object%20Reference) (OtherBodyIndex :type Integer))
  (bind _asbp_player_character (Utilities|Casting|CastToBP_PlayerCharacter OtherActor))
  (if (== (Variables|/Game/BLUE_PRINTS/BP_PlayerCharacter.BP_PlayerCharacter_C|GetDoorInRange _asbp_player_character) self)
    (Variables|/Game/BLUE_PRINTS/BP_PlayerCharacter.BP_PlayerCharacter_C|SetDoorInRange _asbp_player_character 0)))

(event Custom|OpenDoor
  (params (PlayerFacingX :type Float%20%28double-precision%29))
  (Utilities|FlowControl|FlipFlop
    (:A
      (Variables|Default|SetSwingSign (* PlayerFacingX -1.0))
      (Collision|SetCollisionEnabled (Variables|Default|GetDoorBlocker) "NoCollision")
      (bind (_direction _doorangle) (Timeline|TL_OpenDoor Play)
        (:Update
          (Transformation|SetRelativeRotation (Variables|Default|GetHinge) (Math|Rotator|MakeRotator 0.0 0.0 (* _doorangle (Variables|Default|GetSwingSign))) false false))
        (:Finished
          (if (not (Utilities|Enum|Equal(Enum) _direction "Forward"))
            (Collision|SetCollisionEnabled (Variables|Default|GetDoorBlocker) "QueryAndPhysics")))))
    (:B
      (Timeline|TL_OpenDoor Reverse))))

(event EventBeginPlay)

(event Collision|EventActorBeginOverlap
  (params (OtherActor :type Actor%20Object%20Reference)))

(event EventTick
  (params (DeltaSeconds :type Float%20%28single-precision%29)))

(fn ConstructionScript)