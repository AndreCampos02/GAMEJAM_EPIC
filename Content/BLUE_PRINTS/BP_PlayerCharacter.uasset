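; Side-scroller player character that moves along the X axis, opens doors and climbs or descends stairs.
; Enhanced Input drives movement and records facing direction, which is passed to the door in range when interacting.
; Stair inputs send the character to the opposite end point of the nearby stairs via a timeline lerp.
; Movement is disabled during that transition and returns to walking when it finishes.
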(event Custom|UseStairs
  (params (Destination :type Vector))
  (if (not (Variables|Default|GetIsUsingStairs))
    (Variables|Default|SetIsUsingStairs true)
    (Variables|Default|SetStairStart (Transformation|GetActorLocation))
    (Variables|Default|SetStairEnd Destination)
    (Pawn|Components|CharacterMovement|DisableMovement (Variables|Character|GetCharacterMovement))
    (bind _nova_faixa_0 (Timeline|TL_UseStairs PlayFromStart)
      (:Update
        (Transformation|SetActorLocation (Math|Vector|Lerp(Vector) (Variables|Default|GetStairStart) (Variables|Default|GetStairEnd) _nova_faixa_0) false false))
      (:Finished
        (Pawn|Components|CharacterMovement|SetMovementMode (Variables|Character|GetCharacterMovement) "MOVE_Walking" 0)
        (Variables|Default|SetIsUsingStairs false)
        (Development|PrintString "CONTROLE LIBERADO")))))

(event Input|EnhancedActionEvents|EnhancedInputActionIA_MoveHorizontal
  (params (ActionValue :type Float%20%28double-precision%29) (ElapsedSeconds :type Float%20%28double-precision%29) (TriggeredSeconds :type Float%20%28double-precision%29) (InputAction :type Input%20Action%20Object%20Reference :default "/Game/BLUE_PRINTS/input/IA_MoveHorizontal.IA_MoveHorizontal"))
  (if (not (Variables|Default|GetIsUsingStairs))
    (Variables|Default|SetFacingX (Math|Float|SelectFloat 1.0 -1.0 (> ActionValue 0.0)))
    (Pawn|Input|AddMovementInput "1.000000,0.000000,0.000000" ActionValue false)))

(event Input|EnhancedActionEvents|EnhancedInputActionIA_Interact
  (params (ActionValue :type Boolean) (ElapsedSeconds :type Float%20%28double-precision%29) (TriggeredSeconds :type Float%20%28double-precision%29) (InputAction :type Input%20Action%20Object%20Reference :default "/Game/BLUE_PRINTS/input/IA_Interact.IA_Interact"))
  (bind _doorinrange (Variables|Default|GetDoorInRange))
  (:Started
    (Utilities|IsValid _doorinrange
      (:Is%20Valid
        (Default|OpenDoor _doorinrange (Variables|Default|GetFacingX)))
      (:Is%20Not%20Valid
        (Development|PrintString "sem porta")))))

(event Input|EnhancedActionEvents|EnhancedInputActionIA_StairsUp
  (params (ActionValue :type Boolean) (ElapsedSeconds :type Float%20%28double-precision%29) (TriggeredSeconds :type Float%20%28double-precision%29) (InputAction :type Input%20Action%20Object%20Reference :default "/Game/BLUE_PRINTS/input/IA_StairsUp.IA_StairsUp"))
  (bind _stairsatbottom (Variables|Default|GetStairsAtBottom))
  (:Started
    (Utilities|IsValid _stairsatbottom
      (:Is%20Valid
        (CallFunction|UseStairs (Transformation|GetWorldLocation (Variables|/Game/BLUE_PRINTS/BP_BlockoutStairs.BP_BlockoutStairs_C|GetTopPoint _stairsatbottom)))))))

(event Input|EnhancedActionEvents|EnhancedInputActionIA_StairsDown
  (params (ActionValue :type Boolean) (ElapsedSeconds :type Float%20%28double-precision%29) (TriggeredSeconds :type Float%20%28double-precision%29) (InputAction :type Input%20Action%20Object%20Reference :default "/Game/BLUE_PRINTS/input/IA_StairsDown.IA_StairsDown"))
  (bind _stairsattop (Variables|Default|GetStairsAtTop))
  (:Started
    (Utilities|IsValid _stairsattop
      (:Is%20Valid
        (CallFunction|UseStairs (Transformation|GetWorldLocation (Variables|/Game/BLUE_PRINTS/BP_BlockoutStairs.BP_BlockoutStairs_C|GetBottomPoint _stairsattop)))))))

(event EventBeginPlay
  (Input|AddMappingContext (PlayerController|LocalPlayerSubsystems|GetEnhancedInputLocalPlayerSubsystem (Game|GetPlayerController 0)) "/Game/BLUE_PRINTS/input/IMC_SideScroller.IMC_SideScroller" 0 "(bIgnoreAllPressedKeysUntilRelease=True,bForceImmediately=False,bNotifyUserSettings=False)"))

(event Collision|EventActorBeginOverlap
  (params (OtherActor :type Actor%20Object%20Reference)))

(event EventTick
  (params (DeltaSeconds :type Float%20%28single-precision%29)))

(fn ConstructionScript)