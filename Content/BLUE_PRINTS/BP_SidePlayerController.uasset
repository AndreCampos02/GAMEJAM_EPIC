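; Player controller for a side-view camera setup that routes the view through a BP_SideCamera placed in the level.
; On BeginPlay it finds and caches that camera, sets the controlled pawn as its follow target and makes it the view target.
; On possession it retargets the cached camera to the newly possessed pawn, guarded by a validity check.
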(event EventBeginPlay
  (bind _returnvalue (Actor|GetActorOfClass "/Game/BLUE_PRINTS/BP_SideCamera.BP_SideCamera_C"))
  (Variables|Default|SetSideCamera _returnvalue)
  (Utilities|IsValid (Variables|Default|GetSideCamera)
    (:Is%20Valid
      (Default|SetFollowTarget (Variables|Default|GetSideCamera) (Pawn|GetControlledPawn))
      (Game|Player|SetViewTargetwithBlend (Variables|Default|GetSideCamera) 0.0 "VTBlend_Linear" 0.0 false))))

(event EventTick
  (params (DeltaSeconds :type Float%20%28single-precision%29)))

(event EventPossess
  (params (PossessedPawn :type Pawn%20Object%20Reference))
  (bind _sidecamera (Variables|Default|GetSideCamera))
  (Utilities|IsValid _sidecamera
    (:Is%20Valid
      (Default|SetFollowTarget _sidecamera PossessedPawn))))

(fn ConstructionScript)